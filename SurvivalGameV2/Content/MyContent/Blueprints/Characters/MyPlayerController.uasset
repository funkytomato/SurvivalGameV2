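; MyPlayerController is a player controller that sets up the on-screen UI for the local player.
; On BeginPlay, only for a local controller, it creates the PlayerHUD_WBP and WBuffTray widgets, stores references to both and adds them to the viewport.
; Pressing the Inventory input action calls DisplayPlayerMenu on the stored HUD widget.
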(event `self.ReceiveBeginPlay`
  (if (`self.IsLocalPlayerController`)
    (bind _returnvalue (`|CreateWidget` "/Game/MyContent/Blueprints/InventorySystem/UI/PlayerHUD_WBP.PlayerHUD_WBP_C"))
    (bind _output_get (set `self.HUD` _returnvalue))
    (`UserWidget.AddToViewport` _output_get 0)
    (bind _returnvalue_2 (`|CreateWidget` "/Game/MyContent/Blueprints/BuffSystem/UI/W-BuffTray.W-BuffTray_C"))
    (bind _output_get_2 (set `self.TrayHUD` _returnvalue_2))
    (`UserWidget.AddToViewport` _output_get_2 0)))

(event `InputAction|Inventory`
  (params (Key :type "Key Structure"))
  (:`Pressed`
    (`/Game/MyContent/Blueprints/InventorySystem/UI/PlayerHUD_WBP.DisplayPlayerMenu` (`self.HUD`))))

(fn `UserConstructionScript`)