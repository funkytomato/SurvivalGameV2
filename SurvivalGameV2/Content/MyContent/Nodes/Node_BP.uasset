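; Harvestable resource node that gives the player random items from its Resources list as it takes damage.
; Incoming damage is scaled by a DamageTable lookup on the damage type's tool message, then applied to the stat component's health.
; Each damage event shrinks the cube in proportion to remaining health and spawns a Niagara effect.
; Damage accumulates, adding items to player 0's inventory per 100 points and carrying over the remainder.
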(event `self.ReceiveAnyDamage`
  (params (Damage :type "Float (single-precision)") (DamageType :type "DamageType Object Reference") (InstigatedBy :type "Controller Object Reference") (DamageCauser :type "Actor Object Reference"))
  (bind _tooltype (message `/Game/MyContent/Blueprints/IInteractInterface.GetToolType` DamageType))
  (`/Game/MyContent/StatComponent_BP.AffectHealth` (`self.StatComponent_BP`) (* Damage (`BlueprintMapLibrary.Map_Find` (`self.DamageTable`) _tooltype))))

(event `self.StatComponent_BP.OnDamage`
  (params (Health :type "Float (double-precision)") (Damage :type "Float (double-precision)"))
  (`self.RescaleMesh`)
  (bind _output_get (set `self.AccumulatedDamage` (+ Damage (`self.AccumulatedDamage`))))
  (if (> _output_get 100.0)
    (for _ (range (+ (`KismetMathLibrary.FTrunc` (- (/ _output_get 100.0) 1.0)) 1))
      (`/Game/MyContent/Blueprints/InventorySystem/InventorySystem.AddToInventory` (`self.GetComponentByClass` (`GameplayStatics.GetPlayerCharacter` 0) "/Game/MyContent/Blueprints/InventorySystem/InventorySystem.InventorySystem_C") (`KismetArrayLibrary.Array_Random` (`self.Resources`)) 0))
    (set `self.AccumulatedDamage` (mod (`self.AccumulatedDamage`) 100.0))))

(fn `RescaleMesh`
  (bind _statcomponent_bp (`self.StatComponent_BP`))
  (`SceneComponent.SetRelativeScale3D` (`self.Cube`) (* (`self.BaseScale`) (`KismetMathLibrary.NormalizeToRange` (`/Game/MyContent/StatComponent_BP.Health` _statcomponent_bp) 0.0 (`/Game/MyContent/StatComponent_BP.MaxHealth` _statcomponent_bp))))
  (`NiagaraFunctionLibrary.SpawnSystemAtLocation` (`self.NiagaraEffect`) (`self.K2_GetActorLocation`)))

(fn `UserConstructionScript`
  (set `self.BaseScale` (`SceneComponent.RelativeScale3D` (`self.Cube`))))