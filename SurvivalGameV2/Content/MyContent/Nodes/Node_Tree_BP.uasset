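; Tree node Blueprint, built on a parent class, that topples and clears its trunk when its health runs out.
; On health depletion from StatComponent_BP, the mesh starts simulating physics, then after a short delay gets a random, mass-scaled, mostly horizontal impulse.
; A timer later destroys the mesh component.
; RescaleMesh only spawns a Niagara effect at the actor's location, while begin play, overlap and tick defer to the parent.
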(event `self.ReceiveBeginPlay`
  (`parent.ReceiveBeginPlay`))

(event `self.ReceiveActorBeginOverlap`
  (params (OtherActor :type "Actor Object Reference"))
  (`parent.ReceiveActorBeginOverlap` OtherActor))

(event `self.ReceiveTick`
  (params (DeltaSeconds :type "Float (single-precision)"))
  (`parent.ReceiveTick` DeltaSeconds))

(event `self.StatComponent_BP.OnDepletedHealth`
  (bind _mesh (`self.Mesh`))
  (`PrimitiveComponent.SetSimulatePhysics` _mesh true)
  (`KismetSystemLibrary.Delay` 0.5)
  (`PrimitiveComponent.AddImpulse` _mesh (* (`KismetMathLibrary.RandomUnitVector`) (500.0 500.0 50.0) (`PrimitiveComponent.GetMass` (`self.Mesh`))) "None" false)
  (`KismetSystemLibrary.K2_SetTimerDelegate` (delegate `ClearTrunk`) 5.0))

(event `ClearTrunk`
  (`ActorComponent.K2_DestroyComponent` (`self.Mesh`)))

(fn `RescaleMesh`
  (`NiagaraFunctionLibrary.SpawnSystemAtLocation` (`self.NiagaraEffect`) (`self.K2_GetActorLocation`)))

(fn `UserConstructionScript`
  (`parent.UserConstructionScript`))