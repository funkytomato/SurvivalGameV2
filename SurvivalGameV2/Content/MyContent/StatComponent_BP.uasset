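; Stat component that tracks its owning actor's health and destroys that actor when health runs out.
; AffectHealth subtracts the given value, clamps the result between zero and MaxHealth, runs IsAlive, then broadcasts OnDamage with the new health and damage.
; IsAlive doubles as the death handler, destroying the owner at zero health, so this happens before OnDamage fires.
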(fn `AffectHealth`
  (params (Value :type "Float (double-precision)"))
  (returns (Output_Get :type "Float (double-precision)"))
  (bind _output_get (set `self.Health` (`KismetMathLibrary.FClamp` (- (`self.Health`) Value) 0.0 (`self.MaxHealth`))))
  (`self.Is Alive`)
  (`self.OnDamage` (`self.Health`) (`local.Value`))
  (return _output_get))

(fn `Is Alive`
  (returns (IsAlive :type Boolean))
  (if (> (`self.Health`) 0.0)
    (return true)
    (else
      (`Actor.K2_DestroyActor` (`self.GetOwner`))
      (return false))))