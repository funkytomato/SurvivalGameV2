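; Usable tool item that plays an attack montage and damages whatever the player is aiming at.
; UseItem plays the montage on the first-person mesh or third-person character mesh, and its notify begin calls DealDamage.
; DealDamage sphere traces from the camera along its forward vector, applies damage to a damageable hit actor and prints the result.
; GetToolType and LookAt return a fixed enum value and empty text.
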(event `/Game/MyContent/Blueprints/IInteractInterface.UseItem`
  (params (PlayerCharacter :type "Character Object Reference"))
  ;[1 1 1] Use Item
  (bind _asmy_first_person_character (cast `/Game/MyContent/Blueprints/Characters/MyFirstPersonCharacter` PlayerCharacter)
    (:`then`
      (`|PlayMontage` (`/Game/MyContent/Blueprints/Characters/MyFirstPersonCharacter.FirstPersonMesh` _asmy_first_person_character) (`self.Montage to Play`)
        (:`OnNotifyBegin`
          (`self.DealDamage`))))
    (:`CastFailed`
      (bind _asmy_third_person_character (cast `/Game/MyContent/Blueprints/Characters/MyThirdPersonCharacter` PlayerCharacter))
      (`|PlayMontage` (`Character.Mesh` _asmy_third_person_character) (`self.Montage to Play`)
        (:`OnNotifyBegin`
          (`self.DealDamage`))))))

(event `DealDamage`
  (bind _returnvalue (`GameplayStatics.GetPlayerCameraManager` 0))
  (bind _returnvalue_2 (`self.K2_GetActorLocation` _returnvalue))
  ;[1 1 1] Deal Damage
  (bind (_outhit _returnvalue_3) (`KismetSystemLibrary.SphereTraceSingle` :`Start` _returnvalue_2 :`End` (+ _returnvalue_2 (* (`self.GetActorForwardVector` _returnvalue) (`self.Range`))) :`Radius` 20.0 :`TraceChannel` "TraceTypeQuery1" :`DrawDebugType` "ForDuration"))
  (if _returnvalue_3
    (bind (_bblockinghit _binitialoverlap _time _distance _location _impactpoint _normal _impactnormal _physmat _hitactor) (`GameplayStatics.BreakHitResult` _outhit))
    (if (`Actor.bCanBeDamaged` _hitactor)
      (bind _returnvalue_4 (`GameplayStatics.ApplyDamage` _hitactor (`self.BaseDamage`) (`self.GetInstigatorController`) self (`self.Damage Type Class`)))
      (`KismetSystemLibrary.PrintString` (`KismetStringLibrary.Concat_StrStr` "Damage:" (`KismetStringLibrary.Conv_DoubleToString` _returnvalue_4))))))

(fn `GetToolType`
  (returns (ToolType :type "/Game/MyContent/Tools/EToolType Enum"))
  (return "NewEnumerator0"))

(fn `LookAt`
  (returns (message :type Text))
  (return ""))

(fn `UserConstructionScript`)